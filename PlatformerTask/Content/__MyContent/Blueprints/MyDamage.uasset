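; MyDamage is an unfinished damage volume actor aimed at the player-tagged ThirdPersonCharacter.
; On overlap begin it stores the player, flags InsideVolume and runs StartDamage, which sets accumulated damage to InstantDamage capped at MaxDamage without applying it.
; Tick calls ContinueDamage while the flag is set, but that function is empty.
; Overlap end only casts the actor, so the flag is never cleared.
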(event `self.ReceiveTick`
  (params (DeltaSeconds :type "Float (single-precision)"))
  (if (`self.Inside Volume`)
    (`self.Continue Damage`)))

(event `self.collision volume.OnComponentBeginOverlap`
  (params (OverlappedComponent :type "PrimitiveComponent Object Reference") (OtherActor :type "Actor Object Reference") (OtherComp :type "PrimitiveComponent Object Reference") (OtherBodyIndex :type Integer) (bFromSweep :type Boolean) (SweepResult :type "HitResult Structure (by ref)"))
  (if (`self.ActorHasTag` OtherActor "Tag_Player")
    (bind _asthird_person_character (cast `/Game/ThirdPersonBP/Blueprints/ThirdPersonCharacter` OtherActor))
    (set `self.Inside Volume` true)
    (set `self.Player` _asthird_person_character)
    (`self.Start Damage`)))

(event `self.collision volume.OnComponentEndOverlap`
  (params (OverlappedComponent :type "PrimitiveComponent Object Reference") (OtherActor :type "Actor Object Reference") (OtherComp :type "PrimitiveComponent Object Reference") (OtherBodyIndex :type Integer))
  (if (`self.ActorHasTag` OtherActor "Tag_Player")
    (cast `/Game/ThirdPersonBP/Blueprints/ThirdPersonCharacter` OtherActor)))

(fn `Continue Damage`)

(fn `Start Damage`
  (bind _output_get (set `self.Accum Damage` (`self.Instant Damage`)))
  (if (> _output_get (`self.Max Damage`))
    (set `self.Accum Damage` (`self.Max Damage`))))

(fn `UserConstructionScript`)