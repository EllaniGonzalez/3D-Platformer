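; Platform actor that starts moving along a spline automatically when play begins.
; The MovePlatform timeline scales its TravelDistance by spline length to set the mesh's location, roll and yaw, keeping pitch at zero.
; When the timeline finishes, ReversePlatform plays it backwards toward the start.
; Box overlap events cast to ThirdPersonCharacter but trigger no further action.
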(event `self.ReceiveBeginPlay`
  (bind _spline (`self.Spline`))
  (bind (_returnvalue_roll _returnvalue_pitch _returnvalue_yaw) (`KismetMathLibrary.BreakRotator` (`SplineComponent.GetRotationAtDistanceAlongSpline` (`self.Spline`) 0.0 "World")))
  ;[1 1 1] Rotation of Platform
  (`SceneComponent.K2_SetRelativeRotation` (`self.StaticMesh`) (`KismetMathLibrary.MakeRotator` _returnvalue_roll 0.0 _returnvalue_yaw) false false)
  ;[1 1 1] Moving Platform Along Spline
  (bind (_direction _travel_distance) (`Timeline|Move Platform` :!label _label)
    (:`Update`
      (bind _returnvalue (* _travel_distance (`SplineComponent.GetSplineLength` (`self.Spline`))))
      (`SceneComponent.K2_SetWorldLocation` (`self.StaticMesh`) (`SplineComponent.GetLocationAtDistanceAlongSpline` _spline _returnvalue "World") false false)
      (bind (_returnvalue_roll_2 _returnvalue_pitch_2 _returnvalue_yaw_2) (`KismetMathLibrary.BreakRotator` (`SplineComponent.GetRotationAtDistanceAlongSpline` _spline _returnvalue "World")))
      (`SceneComponent.K2_SetRelativeRotation` (`self.StaticMesh`) (`KismetMathLibrary.MakeRotator` _returnvalue_roll_2 0.0 _returnvalue_yaw_2) false false))
    (:`Finished`
      (`self.Reverse Platform`))))

(event `self.Box.OnComponentBeginOverlap`
  (params (OverlappedComponent :type "PrimitiveComponent Object Reference") (OtherActor :type "Actor Object Reference") (OtherComp :type "PrimitiveComponent Object Reference") (OtherBodyIndex :type Integer) (bFromSweep :type Boolean) (SweepResult :type "HitResult Structure (by ref)"))
  ;[1 1 1] Moving Platform Along Spline
  (cast `/Game/ThirdPersonBP/Blueprints/ThirdPersonCharacter` OtherActor))

(event `Reverse Platform`
  ;[1 1 1] Moving Platform Along Spline
  (goto _label :!via `Reverse`))

(event `self.Box.OnComponentEndOverlap`
  (params (OverlappedComponent :type "PrimitiveComponent Object Reference") (OtherActor :type "Actor Object Reference") (OtherComp :type "PrimitiveComponent Object Reference") (OtherBodyIndex :type Integer))
  ;[1 1 1] Return to Starting Position
  (cast `/Game/ThirdPersonBP/Blueprints/ThirdPersonCharacter` OtherActor))

(fn `UserConstructionScript`)