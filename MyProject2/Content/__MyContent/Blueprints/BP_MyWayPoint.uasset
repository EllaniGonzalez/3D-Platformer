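; A moving platform actor with configurable mesh and material that travels along a list of waypoint actors.
; On BeginPlay it hides the waypoints and starts moving, with Start and Stop functions for control.
; A timeline at a configurable rate lerps its relative location between the current and next waypoint world positions.
; The timeline's event advances to the next segment or, at path end, jumps back to the first if Loop is set.
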(event `self.ReceiveBeginPlay`
  ;[1 1 1] Comment
  (for _array_element (`self.Way Points`)
    (`self.SetActorHiddenInGame` _array_element true)
    (`self.Platform Start`)))

(event `Platform Start`
  (bind _motion_timeline (`self.Motion Timeline`))
  ;[1 1 1] Comment
  (`self.Set First Waypoint`)
  (`TimelineComponent.SetPlayRate` _motion_timeline (`self.Rate`))
  (`TimelineComponent.PlayFromStart` _motion_timeline))

(fn `Path Is Finished`
  (returns (`Is Finished` :type Boolean))
  ;[1 1 1] Comment
  (return (== (`self.Next Waypoint Index`) (- (`KismetArrayLibrary.Array_Length` (`self.Way Points`)) 1))))

(fn `Set First Waypoint`
  ;[1 1 1] Comment
  (set `self.Current Waypoint Intex` 0)
  (set `self.Next Waypoint Index` 1)
  (`self.Set Position`))

(fn `Set Next Waypoint`
  ;[1 1 1] Comment
  (bind _result (`/Engine/EditorBlueprintResources/StandardMacros.IncrementInt` (`self.Current Waypoint Intex`))
    (:`  `
      (set `self.Next Waypoint Index` (+ _result 1))
      (`self.Set Position`))))

(fn `Set Position`
  (bind _way_points (`self.Way Points`))
  ;[1 1 1] Comment
  (set `self.Current Waypoint Position` (`self.K2_GetActorLocation` (`|GetArrayItem` _way_points (`self.Current Waypoint Intex`))))
  (set `self.Next Waypoint Position` (`self.K2_GetActorLocation` (`|GetArrayItem` _way_points (`self.Next Waypoint Index`)))))

(fn `Start`
  ;[1 1 1] Run Custom Event
  (`self.Platform Start`))

(fn `Stop`
  ;[1 1 1] Comment
  (`TimelineComponent.Stop` (`self.Motion Timeline`)))

(fn `UserConstructionScript`
  (bind _platform_mesh (`self.Platform Mesh`))
  (`StaticMeshComponent.SetStaticMesh` _platform_mesh (`self.Static Mesh`))
  (`PrimitiveComponent.SetMaterial` _platform_mesh 0 (`self.Material`)))