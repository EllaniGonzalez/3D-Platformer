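; BP_MySplinePlatform is a platform actor whose mesh travels along a spline path.
; The construction script applies the mesh and material from variables to the platform mesh.
; BeginPlay calls PlatformStart, which plays a timeline from the start.
; Each update scales the timeline's SplineDistance track by spline length and moves the mesh to that world-space point without sweeping.
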(event `Platform Start`
  (bind _spline (`self.Spline`))
  ;[1 1 1] Set Platform Mesh Location
  (bind (_direction _spline_distance) (`Timeline|Motion Timeline` :!via `PlayFromStart`)
    (:`Update`
      (`SceneComponent.K2_SetWorldLocation` (`self.Platfrom mesh`) (`SplineComponent.GetLocationAtDistanceAlongSpline` _spline (* _spline_distance (`SplineComponent.GetSplineLength` _spline)) "World") false false))))

(event `self.ReceiveBeginPlay`
  ;[1 1 1] Comment
  (`self.Platform Start`))

(fn `UserConstructionScript`
  (bind _platfrom_mesh (`self.Platfrom mesh`))
  ;[1 1 1] Comment
  (`StaticMeshComponent.SetStaticMesh` _platfrom_mesh (`self.Static Mesh`))
  (`PrimitiveComponent.SetMaterial` _platfrom_mesh 0 (`self.Material`)))