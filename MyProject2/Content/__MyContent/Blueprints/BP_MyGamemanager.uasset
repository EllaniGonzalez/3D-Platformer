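; Game manager Blueprint that owns the game state (Running, Win, Lose, Abandon) and the matching UI.
; Init creates the health, won, lost and abandon widgets, initializes the player and enters Running.
; SetState acts only on a change, hiding UI, then showing either the HUD without mouse or the matching end screen with mouse.
; ResetGame moves the player to the first PlayerStart and reruns Init, creating the widgets again.
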(fn `create UI`
  ;[1 1 1] Comment
  (bind _returnvalue (`|CreateWidget` "/Game/__MyContent/UI/Widget_Abandon.Widget_Abandon_C"))
  (bind _output_get (set `self.Widget Abandon` _returnvalue))
  (`UserWidget.AddToViewport` _output_get 0)
  (bind _returnvalue_2 (`|CreateWidget` "/Game/__MyContent/UI/Widget_Lost.Widget_Lost_C"))
  (bind _output_get_2 (set `self.Widget Lost` _returnvalue_2))
  (`UserWidget.AddToViewport` _output_get_2 0)
  (bind _returnvalue_3 (`|CreateWidget` "/Game/__MyContent/UI/Widget_Won.Widget_Won_C"))
  (bind _output_get_3 (set `self.Widget Won` _returnvalue_3))
  (`UserWidget.AddToViewport` _output_get_3 0)
  (bind _returnvalue_4 (`|CreateWidget` "/Game/__MyContent/UI/Widget_Health.Widget_Health_C"))
  (bind _output_get_4 (set `self.Widget Health` _returnvalue_4))
  (`UserWidget.AddToViewport` _output_get_4 0))

(fn `Get State`
  (returns (State :type "/Game/__MyContent/Blueprints/BP_MyGameStates Enum"))
  ;[1 1 1] Get Current Game State
  (return (`self.Current Game State`)))

(fn `Init`
  ;[1 1 1] Comment
  (`self.create UI`)
  (`/Game/ThirdPersonBP/Blueprints/ThirdPersonCharacter.Init` (`self.My Player`))
  (`self.Set State` "NewEnumerator0"))

(fn `Reset Game`
  (locals (NewLocalVar_0 :type "/Game/__MyContent/Blueprints/BP_MyGamemanager Object Reference"))
  ;[1 1 1] To Be Continued
  (bind _outactors (`GameplayStatics.GetAllActorsOfClass` "/Script/Engine.PlayerStart"))
  (`self.K2_SetActorLocation` (`self.My Player`) (`self.K2_GetActorLocation` (`|GetArrayItem` _outactors)) false false)
  (`self.Init`))

(fn `Set State`
  (params (`New State` :type "/Game/__MyContent/Blueprints/BP_MyGameStates Enum" :default "NewEnumerator4"))
  ;[1 1 1] Changing State
  (if (`|EnumInequality` `New State` (`self.Current Game State`))
    (`/Game/__MyContent/Blueprints/BP_MyFunctionLibrary.Hide UI`)
    (bind _output_get (set `self.Current Game State` `New State`))
    (switch `/Game/__MyContent/Blueprints/BP_MyGameStates` _output_get
      (:`NewEnumerator0`
        (`/Game/__MyContent/Blueprints/BP_MyFunctionLibrary.Show Mouse` false)
        (`self.Show HUD` true))
      (:`NewEnumerator1`
        (`Widget.SetVisibility` (`self.Widget Won`) "Visible")
        (`/Game/__MyContent/Blueprints/BP_MyFunctionLibrary.Show Mouse` true :!label _label))
      (:`NewEnumerator2`
        (`Widget.SetVisibility` (`self.Widget Lost`) "Visible")
        (goto _label))
      (:`NewEnumerator3`
        (`Widget.SetVisibility` (`self.Widget Abandon`) "Visible")
        (goto _label)))))

(fn `Show HUD`
  (params (`Visible Input` :type Boolean))
  (bind _widget_health (`self.Widget Health`))
  ;[1 1 1] Comment
  (if `Visible Input`
    (`Widget.SetVisibility` _widget_health "Visible")
    (else
      (`Widget.SetVisibility` _widget_health "Hidden"))))

(fn `UserConstructionScript`)